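; Pawn Blueprint that tints its mesh to show its current power level during gameplay.
; The construction script creates a dynamic material instance from the mesh's first material and stores it as PowerMaterial.
; The PowerChangeEffect event sets that material's DiffuseColor, blending from red when empty to cyan at initial power using the current-to-initial power ratio.
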(event `self.ReceiveTick`
  (params (DeltaSeconds :type "Float (single-precision)")))

(event `self.PowerChangeEffect`
  ;[1 1 1] Update character Color based on Power Level
  (`MaterialInstanceDynamic.SetVectorParameterValue` (`self.PowerMaterial`) "DiffuseColor" (`KismetMathLibrary.LinearColorLerp` (struct :`R` 1.0 :`A` 1.0) (struct :`G` 1.0 :`B` 1.0 :`A` 1.0) (/ (`self.GetCurrentPower`) (`self.GetInitialPower`)))))

(fn `UserConstructionScript`
  (bind _mesh (`self.Mesh`))
  ;[1 1 1] Setup Dynamic Material to Change Colors during Gameplay
  (bind _returnvalue (`PrimitiveComponent.CreateDynamicMaterialInstance` _mesh 0 (`|GetArrayItem` (`MeshComponent.GetMaterials` _mesh)) "None"))
  (set `self.PowerMaterial` _returnvalue))